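; MenuMonitor_BP is an interactable monitor actor that serves as a camera view target with a mouse cursor, apparently for an in-world menu.
; StartTask blends the view to the monitor, switches input to Game and UI, and binds the Player_BP right-click to GoBack.
; GoBack blends back to the player character, restores game-only input, hides the cursor and prints a debug string.
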(event `/Game/Blueprints/_Interfaces/TaskInterface.StartTask`
  (bind _returnvalue (`GameplayStatics.GetPlayerController` 0))
  (`PlayerController.SetViewTargetWithBlend` (`GameplayStatics.GetPlayerController` 0) self 1.0 "VTBlend_Linear" 0.0 false)
  (bind _asplayer_bp (cast `/Game/Blueprints/Player/Player_BP` (`GameplayStatics.GetPlayerCharacter` 0)))
  (`self.BindEventsToMouse` _asplayer_bp)
  (`WidgetBlueprintLibrary.SetInputMode_GameAndUIEx` _returnvalue null "LockOnCapture")
  (set `PlayerController.bShowMouseCursor` true _returnvalue))

(event `BindEventsToMouse`
  (params (Player :type "/Game/Blueprints/Player/Player_BP Object Reference"))
  (add `/Game/Blueprints/Player/Player_BP.RightClick` Player (delegate `GoBack`)))

(event `GoBack`
  (bind _returnvalue (`GameplayStatics.GetPlayerController` 0))
  (`PlayerController.SetViewTargetWithBlend` (`GameplayStatics.GetPlayerController` 0) (`GameplayStatics.GetPlayerCharacter` 0) 1.0 "VTBlend_Linear" 0.0 false)
  (`KismetSystemLibrary.PrintString` "Hello")
  (`WidgetBlueprintLibrary.SetInputMode_GameOnly` _returnvalue)
  (set `PlayerController.bShowMouseCursor` false _returnvalue))

(fn `UserConstructionScript`)