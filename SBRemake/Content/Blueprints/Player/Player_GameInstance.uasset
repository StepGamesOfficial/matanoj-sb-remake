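; Player game instance that runs the demo's repair-task loop and manages Discord Rich Presence.
; SetUpDEMO builds a queue of randomly picked tagged task actors, destroys the unpicked ones and activates the first task.
; Each completion advances the queue with type-specific audio, and a resettable DoOnce wakes Chica and Bonnie after the first.
; An empty queue prompts a return to the office and activates the monitor.
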(event `Set Up DEMO`
  (`|ExecutionSequence`
    (:`then_0`
      (`KismetArrayLibrary.Array_Clear` (`self.TaskActorQueue`)) ; Reset all values
      (`KismetArrayLibrary.Array_Clear` (`self._TaskActors`))
      (`KismetArrayLibrary.Array_Clear` (`self.TaskTypes`))
      (`BlueprintMapLibrary.Map_Clear` (`self.TasksAvailable`))
      (set `self._rndTask` null))
    (:`then_1`
      (`KismetArrayLibrary.Array_Add` (`self.TaskTypes`) "NewEnumerator5"))
    (:`then_2`
      ;[1 1 1] Pre-emptively get ALL actors of each task type
      (for _array_element (`|MakeArray` "task-vent" "task-pipe" "task-breakers" :!type "Name")
        (bind _outactors (`GameplayStatics.GetAllActorsWithTag` _array_element))
        (`BlueprintMapLibrary.Map_Add` (`self.TasksAvailable`) _array_element (make `/Game/Structs/TaskActors` _outactors))))
    (:`then_3`
      (set `self.MapVariant` (`KismetMathLibrary.RandomIntegerInRange` 0))
      (for _ (range 5)
        (bind _output_get (set `self.NewRandomTaskT` (`KismetArrayLibrary.Array_Random` (`|MakeArray` "NewEnumerator2" "NewEnumerator1" :!type "/Game/Enums/ETaskType Enum"))))
        (`KismetArrayLibrary.Array_Add` (`self.TaskTypes`) _output_get) ; FIX !!!!
      )
      (for (_array_element_2 _array_index) (`self.TaskTypes`)
        (bind _value (`BlueprintMapLibrary.Map_Find` (`self.TaskTags`) _array_element_2))
        (bind _output_get_2 (set `self._TaskActors` (break `/Game/Structs/TaskActors` (`BlueprintMapLibrary.Map_Find` (`self.TasksAvailable`) _value))))
        (bind _output_get_3 (set `self._rndTask` (`KismetArrayLibrary.Array_Random` _output_get_2)))
        (`KismetArrayLibrary.Array_Add` (`self.TaskActorQueue`) _output_get_3)
        (`KismetArrayLibrary.Array_RemoveItem` _output_get_2 _output_get_3)
        (`BlueprintMapLibrary.Map_Add` (`self.TasksAvailable`) _value (make `/Game/Structs/TaskActors` (`self._TaskActors`))))
      (bind _values (`BlueprintMapLibrary.Map_Values` (`self.TasksAvailable`)))
      (for _array_element_3 _values
        (for _array_element_4 (break `/Game/Structs/TaskActors` _array_element_3)
          (`Actor.K2_DestroyActor` _array_element_4)))
      (message `/Game/Blueprints/_Interfaces/TaskInterface.ActivateTask` (`|GetArrayItem` (`self.TaskActorQueue`))))
    (:`then_4`
      (bind _outactors_2 (`GameplayStatics.GetAllActorsOfClass` "/Game/Blueprints/Monitor_BP.Monitor_BP_C"))
      (bind _output (`|GetArrayItem` _outactors_2))
      (`/Engine/EditorBlueprintResources/StandardMacros.IsValid` _output
        (:`Is Valid`
          (set `self.Monitor` _output))))
    (:`then_5`
      (`self.ResetDoonceChica`))))

(event `self.ReceiveInit`
  (bind _returnvalue (`|GenericCreateObject` "/Script/DiscordRpc.DiscordRpc" self))
  (bind _output_get (set `self.Discord REF` _returnvalue))
  (`DiscordRpc.Initialize` _output_get "1280896497453371442" false ""))

(event `LastTaskCompleted`
  (bind _taskactorqueue (`self.TaskActorQueue`))
  (`|ExecutionSequence`
    (:`then_0`
      ;[1 1 1] On task finished
      (switch `name` (`|GetArrayItem` (`Actor.Tags` (`|GetArrayItem` (`self.TaskActorQueue`))) 1)
        (:`task-vent`
          (`KismetSystemLibrary.Delay` 0.5)
          (`GameplayStatics.PlaySound2D` "/Game/Sounds/Dubbing/Gregory/ENG/Nice__this_vent_is_repaired.Nice__this_vent_is_repaired" 1.0 1.0 0.0 null null))
        (:`task-pipe`
          (`KismetSystemLibrary.Delay` 0.5)
          (`GameplayStatics.PlaySound2D` "/Game/Sounds/Dubbing/Gregory/ENG/Nice__no_more_gas_leaks.Nice__no_more_gas_leaks" 1.0 1.0 0.0 null null))))
    (:`then_1`
      (`KismetArrayLibrary.Array_Remove` _taskactorqueue)
      (if (== (`KismetArrayLibrary.Array_Length` _taskactorqueue) 0)
        (`/Engine/EditorBlueprintResources/StandardMacros.DoOnce` false
          (:`Completed`
            (`KismetSystemLibrary.Delay` 4.0)
            (bind _returnvalue (`|CreateWidget` "/Game/CustomWidgets/PopUp_UI.PopUp_UI_C" null "All tasks completed! \nReturn to the office, \nand restart all generators." 0.2 :!label _label))
            (`UserWidget.AddToViewport` _returnvalue 0)
            (`/Engine/EditorBlueprintResources/StandardMacros.DoOnce` false
              (:`Completed`
                (`GameplayStatics.PlaySound2D` "/Game/Sounds/Ventilation/Footstep_Metal_3.Footstep_Metal_3" 1.2 0.1 0.0 null null)
                (`/Game/Blueprints/Monitor_BP.Activate Monitor` (`self.Monitor`))
                (`KismetSystemLibrary.Delay` 5.0)
                (goto _label)))))
        (else
          (message `/Game/Blueprints/_Interfaces/TaskInterface.ActivateTask` (`|GetArrayItem` _taskactorqueue))
          (`/Engine/EditorBlueprintResources/StandardMacros.DoOnce` false :!label _label_2
            (:`Completed`
              (bind _outactors (`GameplayStatics.GetAllActorsOfClass` "/Game/Blueprints/AI/Animatronic_Base_BP.Animatronic_Base_BP_C"))
              (bind _output (`|GetArrayItem` _outactors))
              (`/Engine/EditorBlueprintResources/StandardMacros.IsValid` _output
                (:`Is Valid`
                  (`/Game/Blueprints/AI/Animatronic_Base_BP.Initialize chica` _output))
                (:`Is Not Valid`
                  _))
              (bind _outactors_2 (`GameplayStatics.GetAllActorsOfClass` "/Game/Blueprints/AI/Animatronic_Bonnie_BP.Animatronic_Bonnie_BP_C"))
              (bind _output_2 (`|GetArrayItem` _outactors_2))
              (`/Engine/EditorBlueprintResources/StandardMacros.IsValid` _output_2
                (:`Is Valid`
                  (`KismetSystemLibrary.Delay` 0.0)
                  (`/Game/Blueprints/AI/Animatronic_Bonnie_BP.Initialize bonnie` _output_2))))))))))

(event `self.ReceiveShutdown`
  (`DiscordRpc.ClearPresence` (`self.Discord REF`)))

(event `ResetDoonceChica`
  (goto _label_2 :!via `Reset`))