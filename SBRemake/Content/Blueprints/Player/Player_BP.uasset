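; First-person player character with movement, sprint, crouch, pause menu and a flashlight arm viewmodel.
; Timelines drive velocity-scaled walk bob with footsteps, look sway on the arm and sprint pose.
; Sprint stamina doubles as Scaredness, which speeds up random hand shake and forces sprint to stop with heavy breathing when exhausted.
; A camera line trace uses actor tags to message doors or start tasks, which stow the flashlight.
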(event `self.ReceiveBeginPlay`
  (bind _scarednessscene (`self.ScarednessScene`))
  (bind _relativerotation (`SceneComponent.RelativeRotation` _scarednessscene))
  (`|ExecutionSequence`
    (:`then_0`
      (bind _asplayer_game_instance (cast `/Game/Blueprints/Player/Player_GameInstance` (`GameplayStatics.GetGameInstance`)))
      (`/Game/Blueprints/Player/Player_GameInstance.Set Up DEMO` _asplayer_game_instance))
    (:`then_1`
      ;[1 1 1] Footstep animations + Sounds
      (bind (_direction _location) (`Timeline|WalkTimeline` :!via `PlayFromStart`)
        (:`Update`
          (`SceneComponent.K2_SetRelativeLocation` (`self.Viewmodel`) _location false false)
          (if true
            (bind _y (.y _location))
            (`SceneComponent.K2_SetRelativeRotation` (`self.Camera`) (`KismetMathLibrary.MakeRotator` (* _y 0.5) (* (.z _location) 0.5) (* _y 1.0)) false false))
          (if (and (`KismetMathLibrary.NearlyEqual_FloatFloat` (mod (`TimelineComponent.GetPlaybackPosition` (`self.WalkTimeline`)) 2.0) 0.0 0.15) (not (`NavMovementComponent.IsFalling` (`self.CharacterMovement`))))
            (`/Engine/EditorBlueprintResources/StandardMacros.DoOnce` false :!label _label
              (:`Completed`
                (`GameplayStatics.PlaySound2D` "/Game/Sounds/Default_Footstep_Cue.Default_Footstep_Cue" (`KismetMathLibrary.SelectFloat` 0.2 0.3 (`NavMovementComponent.IsCrouching` (`self.CharacterMovement`))) 0.8 0.0 null null)))
            (else
              (goto _label :!via `Reset`))))))
    (:`then_2`
      ;[1 1 1 1 15] SCAREDNESS - vystrašenost (čím vystrašenější -> tím víc se ruka klepe - jen nápad)
      (`TimelineComponent.SetPlayRate` (`self.ScaredAnim`) (* (`self.Scaredness`) 20.0) :!label _label_2)
      (bind (_x _y_2 _z) (`self.Random Values XYZ` -1.0 1.0))
      (bind _output_get (set `self.ArmRotTemp` _relativerotation))
      (bind (_direction_2 _alpha) (`Timeline|ScaredAnim` :!via `PlayFromStart`)
        (:`Update`
          (`SceneComponent.K2_SetRelativeRotation` _scarednessscene (`KismetMathLibrary.MakeRotator` (.roll _relativerotation) (`KismetMathLibrary.Lerp` (.pitch _output_get) _y_2 _alpha) (`KismetMathLibrary.Lerp` (.yaw _output_get) _z _alpha)) false false))
        (:`Finished`
          (goto _label_2))))
    (:`then_3`
      (bind _returnvalue (`|CreateWidget` "/Game/CustomWidgets/GeneratorUI.GeneratorUI_C" (`GameplayStatics.GetPlayerController` 0)))
      (bind _output_get_2 (set `self.GeneratorsUI` _returnvalue))
      (`UserWidget.AddToViewport` _output_get_2 0)
      (`Widget.SetVisibility` _output_get_2 "Collapsed"))))

(event `InputAxis|LookUp`
  (params (AxisValue :type "Float (single-precision)"))
  (bind _rotatescene (`self.RotateScene`))
  (bind (_relativerotation_roll _relativerotation_pitch _relativerotation_yaw) (`KismetMathLibrary.BreakRotator` (`SceneComponent.RelativeRotation` _rotatescene)))
  ;[1 1 1] Lookup/LookRight
  (`self.AddControllerPitchInput` AxisValue)
  (`SceneComponent.K2_AddRelativeRotation` _rotatescene (`KismetMathLibrary.MakeRotator` (* (/ AxisValue 2.0) 1.0)) false false)
  (`SceneComponent.K2_SetRelativeRotation` _rotatescene (`KismetMathLibrary.MakeRotator` (`KismetMathLibrary.ClampAngle` _relativerotation_roll -15.0 25.0) _relativerotation_pitch (`KismetMathLibrary.ClampAngle` _relativerotation_yaw -15.0 20.0)) false false :!label _label_3)
  (bind (_direction _lerp) (`Timeline|BackToDefault` :!via `PlayFromStart`)
    (:`Update`
      (`SceneComponent.K2_SetRelativeRotation` _rotatescene (`KismetMathLibrary.RLerp` (`SceneComponent.RelativeRotation` _rotatescene) (struct) _lerp true) false false))))

(event `InputAxis|LookRight`
  (params (AxisValue :type "Float (single-precision)"))
  ;[1 1 1] Lookup/LookRight
  (`self.AddControllerYawInput` AxisValue)
  (`SceneComponent.K2_AddRelativeRotation` (`self.RotateScene`) (`KismetMathLibrary.MakeRotator` 0.0 0.0 (/ AxisValue 1.7)) false false)
  (goto _label_3))

(event `self.ReceiveTick`
  (params (DeltaSeconds :type "Float (single-precision)"))
  ;[1 1 1] Event Tick
  (`TimelineComponent.SetPlayRate` (`self.WalkTimeline`) (`KismetMathLibrary.SelectFloat` 0.0 (+ (/ (`KismetMathLibrary.VSize` (`self.GetVelocity`)) 100.0) 0.1) (`NavMovementComponent.IsFalling` (`self.CharacterMovement`)))))

(event `InputAction|PauseGame` :paused true
  (params (Key :type "Key Structure"))
  (bind _returnvalue (`GameplayStatics.GetPlayerController` 0))
  ;[1 1 1] Pause Game
  (:`Pressed`
    (`GameplayStatics.SetGamePaused` true)
    (bind _returnvalue_2 (`|CreateWidget` "/Game/CustomWidgets/Menu/PauseMenu.PauseMenu_C" _returnvalue))
    (bind _output_get (set `self.PauseWidget` _returnvalue_2))
    (`UserWidget.AddToViewport` _returnvalue_2 0)
    (`UserWidget.AddToViewport` _output_get 0)
    (`WidgetBlueprintLibrary.SetInputMode_UIOnlyEx` _returnvalue _returnvalue_2)
    (set `PlayerController.bShowMouseCursor` true _returnvalue)))

(event `InputAxis|WalkForward`
  (params (AxisValue :type "Float (single-precision)"))
  ;[1 1 1] Basic Input
  (`self.AddMovementInput` (`self.GetActorForwardVector`) AxisValue))

(event `InputAxis|WalkRight`
  (params (AxisValue :type "Float (single-precision)"))
  ;[1 1 1] Basic Input
  (`self.AddMovementInput` (`self.GetActorRightVector`) AxisValue))

(event `InputAction|Interact`
  (params (Key :type "Key Structure"))
  (bind (_start _end) (`self.GetTraceFromCamera` 300.0))
  ;[1 1 1] Interaction
  (:`Pressed`
    (bind _outhit (`KismetSystemLibrary.LineTraceSingleForObjects` _start _end (`|MakeArray` "ObjectTypeQuery1" "ObjectTypeQuery2" "ObjectTypeQuery3" :!type "EObjectTypeQuery Enum")))
    (bind (_bblockinghit _binitialoverlap _time _distance _location _impactpoint _normal _impactnormal _physmat _hitactor) (`GameplayStatics.BreakHitResult` _outhit))
    (`/Engine/EditorBlueprintResources/StandardMacros.IsValid` _hitactor
      (:`Is Valid`
        (switch `name` (`|GetArrayItem` (`Actor.Tags` _hitactor))
          (:`door`
            (message `/Game/Blueprints/_Interfaces/DoorInterface.Toggle Door` _hitactor))
          (:`task`
            (bind _result (message `/Game/Blueprints/_Interfaces/TaskInterface.Get Is Activated` _hitactor))
            (if _result
              (set `self.IsInTask` true)
              (if (`self.FlashlightOut`)
                (`self.ForceHideFlashlight`)
                (`KismetSystemLibrary.Delay` 0.4))
              (message `/Game/Blueprints/_Interfaces/TaskInterface.StartTask` _hitactor))))))))

(event `self.OnLanded`
  (params (Hit :type "HitResult Structure (by ref)"))
  ;[1 1 1] On Landed
  (`GameplayStatics.PlaySound2D` "/Game/Sounds/Default_Footstep_Cue.Default_Footstep_Cue" 1.3 0.8 0.0 null null)
  (if (`self.IsSprinting`)
    (`self.Play/ReverseSprintTimeline` true)))

(event `InputAction|Crouch`
  (params (Key :type "Key Structure"))
  (bind _camera (`self.Camera`))
  ;[1 1 1] Crouch
  (:`Pressed`
    (bind _isa (`/Engine/EditorBlueprintResources/StandardMacros.FlipFlop`)
      (:`A`
        (`self.Crouch`)
        (`self.Play/ReverseSprintTimeline` false)
        (`SceneComponent.K2_SetRelativeLocation` _camera (0.0 0.0 30.0) false false))
      (:`B`
        (`self.UnCrouch`)
        (`SceneComponent.K2_SetRelativeLocation` _camera (0.0 0.0 50.0) false false)))
    (set `self.IsCrouched` _isa)))

(event `InputAction|Sprint`
  (params (Key :type "Key Structure"))
  (bind _charactermovement (`self.CharacterMovement`))
  (bind _stamina (`self.Stamina`))
  ;[1 1 1] Sprinting
  (:`Pressed`
    (if (not (or (`self.IsCrouched`) (< (`KismetMathLibrary.VSize` (`MovementComponent.Velocity` (`self.CharacterMovement`))) 100.0)))
      (set `self.IsSprinting` true)
      (set `CharacterMovementComponent.MaxWalkSpeed` 550.0 _charactermovement)
      (set `CharacterMovementComponent.MaxAcceleration` 500.0 _charactermovement)
      (`|ExecutionSequence`
        (:`then_0`
          (bind (_direction _alpha) (`Timeline|Sprint` :!label _label_4)
            (:`Update`
              (`SceneComponent.K2_SetRelativeTransform` (`self.ViewmodelSpringArm`) (`KismetMathLibrary.TLerp` (`KismetMathLibrary.MakeTransform` (0.0 0.0 0.0)) (`KismetMathLibrary.MakeTransform` (0.0 0.0 -15.0) (struct :`Pitch` -30.0 :`Yaw` -30.0)) _alpha) false false))))
        (:`then_1`
          (`TimelineComponent.SetPlayRate` _stamina 1.0)
          (bind (_direction_2 _progress) (`Timeline|Stamina` :!label _label_5)
            (:`Update`
              (set `self.Scaredness` _progress))
            (:`Finished`
              (if (not (`KismetMathLibrary.NearlyEqual_FloatFloat` _progress 0.1))
                (`GameplayStatics.PlaySound2D` "/Game/Sounds/Animatronics/HeavyBreathing.HeavyBreathing" 1.0 1.0 0.0 null null)
                (`self.ForceStopSprint`)
                (`TimelineComponent.SetPlayRate` _stamina 1.5 :!label _label_6)
                (goto _label_5 :!via `Reverse`))))))))
  (:`Released`
    (set `self.IsSprinting` false :!label _label_7)
    (set `CharacterMovementComponent.MaxWalkSpeed` 250.0 _charactermovement)
    (set `CharacterMovementComponent.MaxAcceleration` 1000.0 _charactermovement)
    (`|ExecutionSequence`
      (:`then_0`
        (goto _label_4 :!via `Reverse`))
      (:`then_1`
        (goto _label_6)))))

(event `self.OnJumped`
  ;[1 1 1] Sprinting
  (goto _label_4 :!via `Reverse`))

(event `Play/ReverseSprintTimeline`
  (params (`Play?` :type Boolean :default true))
  ;[1 1 1] Sprinting
  (if `Play?`
    (goto _label_4)
    (else
      (goto _label_4 :!via `Reverse`))))

(event `ForceStopSprint`
  ;[1 1 1] Sprinting
  (goto _label_7))

(event `InputAction|Flashlight`
  (params (Key :type "Key Structure"))
  (bind _viewmodel (`self.Viewmodel`))
  ;[1 1 1] Flashlight
  (:`Pressed`
    (if (not (`self.IsInTask`))
      (`/Engine/EditorBlueprintResources/StandardMacros.DoOnce` false :!label _label_8
        (:`Completed`
          (if (`self.FlashlightOut`)
            (`SkeletalMeshComponent.PlayAnimation` _viewmodel "/Game/Animations/Viewmodel/NEW/unequip_ArmViewmodel_ArmViewmodelAction_001.unequip_ArmViewmodel_ArmViewmodelAction_001" false :!label _label_9)
            (set `self.FlashlightOut` false)
            (`KismetSystemLibrary.Delay` 0.4)
            (`AudioComponent.SetVolumeMultiplier` (`self.FlashlightAudio`) 0.0)
            (`SceneComponent.SetHiddenInGame` (`self.Viewmodel`) true true)
            (goto _label_8 :!via `Reset`)
            (else
              (`SkeletalMeshComponent.PlayAnimation` _viewmodel "/Game/Animations/Viewmodel/NEW/equip_ArmViewmodel_ArmViewmodelAction_001.equip_ArmViewmodel_ArmViewmodelAction_001" false)
              (`SceneComponent.SetHiddenInGame` (`self.Viewmodel`) false true)
              (set `self.FlashlightOut` true)
              (`KismetSystemLibrary.Delay` 0.4)
              (`AudioComponent.SetVolumeMultiplier` (`self.FlashlightAudio`) 0.2)
              (goto _label_8 :!via `Reset`))))))))

(event `ForceHideFlashlight`
  (goto _label_9))

(event `Key|LeftMouseButton`
  (params (Key :type "Key Structure"))
  (:`Pressed`
    (`self.LeftClick`)))

(event `Key|RightMouseButton`
  (params (Key :type "Key Structure"))
  (:`Pressed`
    (`self.RightClick`)))

(fn `Random Values XYZ`
  (params (Min :type "Float (double-precision)") (Max :type "Float (double-precision)"))
  (returns (X :type "Float (double-precision)") (Y :type "Float (double-precision)") (Z :type "Float (double-precision)"))
  (locals (Value :type "Float (double-precision)") (Value1 :type "Float (double-precision)") (Value2 :type "Float (double-precision)"))
  (bind _output_get (set `local.Value` (`KismetMathLibrary.RandomFloatInRange` Min Max)))
  (bind _output_get_2 (set `local.Value1` (`KismetMathLibrary.RandomFloatInRange` Min Max)))
  (bind _output_get_3 (set `local.Value2` (`KismetMathLibrary.RandomFloatInRange` Min Max)))
  (return _output_get _output_get_2 _output_get_3))

(fn `UserConstructionScript`)