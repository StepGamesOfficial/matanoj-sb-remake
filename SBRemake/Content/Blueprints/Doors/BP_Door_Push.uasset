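; Push door Blueprint that swings a Door component open or closed by 90 degrees in yaw when interacted with.
; ToggleDoor calls Interact, which ignores input while the OpenDoor timeline plays and flip-flops between playing and reversing it.
; Timeline alpha drives the rotation, with UseAOpen selecting the swing direction.
; The dot-product check that would set UseAOpen from player facing is disconnected, so it never runs.
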(event `/Game/Blueprints/_Interfaces/DoorInterface.Toggle Door`
  (`self.Interact`))

(event `Interact`
  (if (not (`TimelineComponent.IsPlaying` (`self.OpenDoor`)))
    (`/Engine/EditorBlueprintResources/StandardMacros.FlipFlop`
      (:`A`
        (bind (_direction _alpha) (`Timeline|OpenDoor` :!label _label)
          (:`Update`
            (`SceneComponent.K2_SetRelativeRotation` (`self.Door`) (`KismetMathLibrary.SelectRotator` (`KismetMathLibrary.RLerp` (struct) (struct :`Yaw` -90.0) _alpha) (`KismetMathLibrary.RLerp` (struct) (struct :`Yaw` 90.0) _alpha) (`self.Use A Open?`)) false false))))
      (:`B`
        (goto _label :!via `Reverse`)))))

(fn `UserConstructionScript`)