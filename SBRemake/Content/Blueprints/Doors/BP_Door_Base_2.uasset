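; Base hinged door that toggles open and closed for the player and opens automatically when an animatronic overlaps its box while closed.
; Interact flip-flops a timeline forward or in reverse, ignoring calls while it is playing.
; On opening, a dot product of the arrow and interactor forward vectors picks the 90-degree swing direction.
; The timeline rotates the door and disables its collision during mid-swing.
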(event `/Game/Blueprints/_Interfaces/DoorInterface.Toggle Door`
  (`self.Interact` (`GameplayStatics.GetPlayerCharacter` 0)))

(event `Interact`
  (params (`Who is interacting` :type "Actor Object Reference"))
  (bind _door (`self.Door`))
  (if (not (`TimelineComponent.IsPlaying` (`self.OpenDoor`)))
    (`/Engine/EditorBlueprintResources/StandardMacros.FlipFlop`
      (:`A`
        (set `self.Use A Open?` (< (`KismetMathLibrary.Dot_VectorVector` (`SceneComponent.GetForwardVector` (`self.Arrow`)) (`self.GetActorForwardVector` `Who is interacting`)) 0.0))
        (set `self.Closed` false)
        (bind (_direction _alpha) (`Timeline|OpenDoor` :!label _label)
          (:`Update`
            (`SceneComponent.K2_SetRelativeRotation` _door (`KismetMathLibrary.SelectRotator` (`KismetMathLibrary.RLerp` (struct) (struct :`Yaw` 90.0) _alpha) (`KismetMathLibrary.RLerp` (struct) (struct :`Yaw` -90.0) _alpha) (`self.Use A Open?`)) false false)
            (`PrimitiveComponent.SetCollisionEnabled` _door (select `bool` (and (> _alpha 0.25) (< _alpha 0.9)) :`false` "QueryAndPhysics" :`true` "NoCollision" :!type "ECollisionEnabled Enum")))))
      (:`B`
        (set `self.Closed` true)
        (goto _label :!via `Reverse`)))))

(event `self.Box.OnComponentBeginOverlap`
  (params (OverlappedComponent :type "PrimitiveComponent Object Reference") (OtherActor :type "Actor Object Reference") (OtherComp :type "PrimitiveComponent Object Reference") (OtherBodyIndex :type Integer) (bFromSweep :type Boolean) (SweepResult :type "HitResult Structure (by ref)"))
  (bind _asanimatronic_base_bp (cast `/Game/Blueprints/AI/Animatronic_Base_BP` OtherActor))
  (if (`self.Closed`)
    (`self.Interact` _asanimatronic_base_bp)))

(fn `UserConstructionScript`)