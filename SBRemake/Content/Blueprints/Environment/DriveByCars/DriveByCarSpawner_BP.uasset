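; Ambient drive-by car spawner that loops a random car along a spline path with a distant pass-by sound.
; After a random delay of several seconds, it swaps one static mesh to a random car model rather than spawning actors.
; A timeline moves and rotates the mesh along the spline, then restarts the cycle when finished.
; In parallel, a delayed attenuated sound plays at the spline's 0.5 time point.
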(event `self.ReceiveBeginPlay`
  (bind _path (`self.path`))
  (`KismetSystemLibrary.Delay` (`KismetMathLibrary.RandomFloatInRange` 7.0 12.0) :!label _label)
  (`StaticMeshComponent.SetStaticMesh` (`self.StaticMesh`) (`KismetArrayLibrary.Array_Random` (`|MakeArray` "/Game/Trailer/Assety/Cars/2/SM_SportsCar.SM_SportsCar" "/Game/Trailer/Assety/Cars/2/SM_Hatchback.SM_Hatchback" "/Game/Trailer/Assety/Cars/2/SM_Pickup.SM_Pickup" "/Game/Trailer/Assety/Cars/2/SM_SUV.SM_SUV" :!type "StaticMesh Object Reference")))
  (`|ExecutionSequence`
    (:`then_0`
      (bind (_direction _alpha) (`Timeline|CarTimeline` :!via `PlayFromStart`)
        (:`Update`
          (`SceneComponent.K2_SetWorldLocationAndRotation` (`self.StaticMesh`) (`SplineComponent.GetLocationAtTime` _path _alpha "World" false) (`SplineComponent.GetRotationAtTime` _path _alpha "World" false) false false))
        (:`Finished`
          (goto _label))))
    (:`then_1`
      (`KismetSystemLibrary.Delay` 1.0)
      (`GameplayStatics.PlaySoundAtLocation` "/Game/Sounds/Ambience/Cars/Car_DistantPassBy.Car_DistantPassBy" (`SplineComponent.GetLocationAtTime` (`self.path`) 0.5 "World" false) (struct) 1.0 1.0 0.0 "/Game/Sounds/Attenuation/DistantCar_Att.DistantCar_Att" null null))))

(fn `UserConstructionScript`)