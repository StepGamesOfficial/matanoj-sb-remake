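; Environment light actor that randomly cuts out and comes back on, with a buzzing sound that follows its state.
; On BeginPlay it stores the point light's intensity, then runs an endless loop of randomized delays with longer on periods and generally shorter off periods.
; Each switch sets the light to zero or its stored intensity and lowers or raises the buzz volume to match, without using Tick.
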(event `self.ReceiveBeginPlay`
  (set `self.BaseIntensity` (`LightComponentBase.Intensity` (`self.PointLight`)))
  (`KismetSystemLibrary.Delay` (`KismetMathLibrary.RandomFloatInRange` 5.0 30.0) :!label _label)
  (`LightComponent.SetIntensity` (`self.PointLight`) 0.0)
  (`AudioComponent.SetVolumeMultiplier` (`self.BuzzingSound`) 0.1)
  (`KismetSystemLibrary.Delay` (`KismetMathLibrary.RandomFloatInRange` 0.5 10.0))
  (`LightComponent.SetIntensity` (`self.PointLight`) (`self.BaseIntensity`))
  (`AudioComponent.SetVolumeMultiplier` (`self.BuzzingSound`) 0.7)
  (goto _label))

(fn `UserConstructionScript`)