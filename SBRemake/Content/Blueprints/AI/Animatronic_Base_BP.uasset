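; Animatronic enemy pawn, set up for Chica, that idles in a looping stage animation until initialized, then runs a behavior tree after a random delay.
; UpdateAIStatus mirrors its status enum to the Blackboard.
; Seeing or touching the player, outside one status, changes state and boosts speed, with retriggerable delays adjusting it afterward and a gated alert sound.
; A one-shot Jumpscare event takes the camera, plays a sound and reopens the gameplay level.
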(event `Initialize chica`
  (`KismetSystemLibrary.Delay` (`KismetMathLibrary.RandomFloatInRange` 8.0 17.0))
  (`AIController.RunBehaviorTree` (`AIBlueprintHelperLibrary.GetAIController` self) "/Game/Blueprints/AI/BehaviourTree_Chica.BehaviourTree_Chica")
  (`self.UpdateAIStatus` "NewEnumerator2")
  (`SkeletalMeshComponent.SetAnimationMode` (`self.Mesh`) "AnimationBlueprint"))

(event `self.ReceiveBeginPlay`
  (`SkeletalMeshComponent.PlayAnimation` (`self.Mesh`) "/Game/Animations/Animatronics/Chica/Chica_Stage_FIXED.Chica_Stage_FIXED" true))

(event `self.PawnSensing.OnSeePawn`
  (params (Pawn :type "Pawn Object Reference"))
  (cast `/Game/Blueprints/Player/Player_BP` Pawn)
  (if (`|EnumInequality` (`self.Status`) "NewEnumerator0") :!label _label
    (`SkeletalMeshComponent.SetAnimationMode` (`self.Mesh`) "AnimationBlueprint")
    (`self.UpdateAIStatus` "NewEnumerator3")
    (set `CharacterMovementComponent.MaxWalkSpeed` 450.0 (`self.CharacterMovement`))
    (`|ExecutionSequence`
      (:`then_0`
        (`KismetSystemLibrary.RetriggerableDelay` 3.0)
        (`MovementComponent.StopMovementImmediately` (`self.CharacterMovement`))
        (set `CharacterMovementComponent.MaxWalkSpeed` 370.0 (`self.CharacterMovement`))
        (goto _label_2 :!via `Reset`))
      (:`then_1`
        (`/Engine/EditorBlueprintResources/StandardMacros.DoOnce` false :!label _label_2
          (:`Completed`
            (bind _returnvalue (`GameplayStatics.SpawnSoundAttached` "/Game/Sounds/Animatronics/NightmareJumpscare.NightmareJumpscare" (`self.Mesh`) "None" (0.0 0.0 0.0) (struct) "KeepRelativeOffset" false 0.4 2.0 0.0 "/Game/Sounds/Attenuation/Animatronic_Att.Animatronic_Att" null))
            (`AudioComponent.Play` _returnvalue 0.0))))
      (:`then_2`
        (`KismetSystemLibrary.RetriggerableDelay` 1.5)
        (set `CharacterMovementComponent.MaxWalkSpeed` 300.0 (`self.CharacterMovement`))))))

(event `Jumpscare`
  (`/Engine/EditorBlueprintResources/StandardMacros.DoOnce` false
    (:`Completed`
      (`PlayerController.SetViewTargetWithBlend` (`GameplayStatics.GetPlayerController` 0) self 0.0 "VTBlend_Linear" 0.0 false)
      (`GameplayStatics.PlaySound2D` "/Game/Sounds/Animatronics/SecurityBreachJumpscare.SecurityBreachJumpscare" 1.0 1.0 0.0 null null)
      (`KismetSystemLibrary.Delay` 3.0)
      (`GameplayStatics.OpenLevelBySoftObjectPtr` "/Game/Levels/GAMEPLAY/GAMEPLAY_Demo.GAMEPLAY_Demo" false))))

(event `self.Capsule.OnComponentBeginOverlap`
  (params (OverlappedComponent :type "PrimitiveComponent Object Reference") (OtherActor :type "Actor Object Reference") (OtherComp :type "PrimitiveComponent Object Reference") (OtherBodyIndex :type Integer) (bFromSweep :type Boolean) (SweepResult :type "HitResult Structure (by ref)"))
  (cast `/Game/Blueprints/Player/Player_BP` OtherActor)
  (goto _label))

(fn `UpdateAIStatus`
  (params (`New status` :type "/Game/Enums/EAnimatronicStatus Enum" :default "NewEnumerator0"))
  (`BlackboardComponent.SetValueAsEnum` (`AIBlueprintHelperLibrary.GetBlackboard` (`AIBlueprintHelperLibrary.GetAIController` self)) "Status" `New status`)
  (set `self.Status` `New status`))

(fn `UserConstructionScript`)