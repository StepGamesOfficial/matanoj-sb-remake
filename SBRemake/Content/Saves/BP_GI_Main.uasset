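; Game Instance Blueprint that handles loading and saving of the player's gamma setting through an SGB_Settings save object.
; LoadGamma loads the GammaSave slot or creates a new object, applying r.TonemapperGamma by console command only for a new one.
; SaveGamma writes the slot first, then updates GammaValue in memory if that succeeds.
; LoadGammaSettings returns the cached value when the object is valid.
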(event `LoadGamma`
  (bind _returnvalue (`GameplayStatics.DoesSaveGameExist` (`self.GammaSave`)))
  (if _returnvalue
    (bind _returnvalue_2 (`GameplayStatics.LoadGameFromSlot` (`self.GammaSave`)))
    (bind _assgb_settings (cast `/Game/Saves/SGB_Settings` _returnvalue_2))
    (set `self.SGB_Settings` _assgb_settings)
    (else
      (bind _returnvalue_3 (`GameplayStatics.CreateSaveGameObject` "/Game/Saves/SGB_Settings.SGB_Settings_C"))
      (bind _output_get (set `self.SGB_Settings` _returnvalue_3))
      (`KismetSystemLibrary.ExecuteConsoleCommand` (`KismetTextLibrary.Conv_TextToString` (`|FormatText` "r.TonemapperGamma {x}" (`/Game/Saves/SGB_Settings.GammaValue` _output_get))) (`GameplayStatics.GetPlayerController` 0)))))

(event `SaveGamma`
  (params (GammaValue :type "Float (double-precision)"))
  (bind _returnvalue (`GameplayStatics.SaveGameToSlot` (`self.SGB_Settings`) (`self.GammaSave`)))
  (if _returnvalue
    (set `/Game/Saves/SGB_Settings.GammaValue` GammaValue (`self.SGB_Settings`))))

(fn `LoadGammaSettings`
  (returns (GammaValue :type "Float (double-precision)"))
  (bind _sgb_settings (`self.SGB_Settings`)
    (:`then`
      (return (`/Game/Saves/SGB_Settings.GammaValue` _sgb_settings)))
    (:`else`)))