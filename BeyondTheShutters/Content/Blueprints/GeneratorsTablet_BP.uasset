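; GeneratorsTablet_BP is a tablet actor that opens the player's generators UI when the player walks into its box trigger while it is activated.
; On overlap it shows the Player_BP's GeneratorsUI widget, switches input to UI only with the mouse cursor, and calls OnCreate on the GeneratorUI.
; A DoOnce blocks repeat opening until one second after the player leaves the box.
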(event `self.Box.OnComponentBeginOverlap`
  (params (OverlappedComponent :type "PrimitiveComponent Object Reference") (OtherActor :type "Actor Object Reference") (OtherComp :type "PrimitiveComponent Object Reference") (OtherBodyIndex :type Integer) (bFromSweep :type Boolean) (SweepResult :type "HitResult Structure (by ref)"))
  (bind _returnvalue (`GameplayStatics.GetPlayerController` 0))
  (if (`self.Activated`)
    (bind _asplayer_bp (cast `/Game/Blueprints/Player/Player_BP` OtherActor))
    (`/Engine/EditorBlueprintResources/StandardMacros.DoOnce` false :!label _label
      (:`Completed`
        (bind _generatorsui (`/Game/Blueprints/Player/Player_BP.GeneratorsUI` _asplayer_bp))
        (`Widget.SetVisibility` _generatorsui "Visible")
        (`WidgetBlueprintLibrary.SetInputMode_UIOnlyEx` _returnvalue _generatorsui)
        (set `PlayerController.bShowMouseCursor` true _returnvalue)
        (bind _asgenerator_ui (cast `/Game/CustomWidgets/GeneratorUI` _generatorsui))
        (`/Game/CustomWidgets/GeneratorUI.OnCreate` _asgenerator_ui)))))

(event `self.Box.OnComponentEndOverlap`
  (params (OverlappedComponent :type "PrimitiveComponent Object Reference") (OtherActor :type "Actor Object Reference") (OtherComp :type "PrimitiveComponent Object Reference") (OtherBodyIndex :type Integer))
  (cast `/Game/Blueprints/Player/Player_BP` OtherActor)
  (`KismetSystemLibrary.Delay` 1.0)
  (goto _label :!via `Reset`))

(fn `UserConstructionScript`)